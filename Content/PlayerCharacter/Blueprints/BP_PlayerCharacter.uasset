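; Player character Blueprint that maps input to movement, camera rotation, walk, sprint, light attack and lock-on targeting.
; Axis events pair forward with strafe and turn with look-up for mouse or gamepad, while actions forward to movement, combat and targeting calls.
; X-Ray toggles a timeline forward and back to animate a post-process material parameter collection's alpha.
; Keys 1 and 2 switch slow motion on and off through global time dilation.
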(event EventTick
  (params (DeltaSeconds :type Float%20%28single-precision%29)))

(event Input|ActionEvents|InputActionSprint
  (params (Key :type Key%20Structure :default "None"))
  ;[0 0 0] Walk - Sprint
  (:Pressed
    (Class|PlayerCharacter|Sprint :!label _label))
  (:Released
    (goto _label Released)))

(event Input|ActionEvents|InputActionWalk
  (params (Key :type Key%20Structure :default "None"))
  ;[0 0 0] Walk - Sprint
  (:Pressed
    (Class|PlayerCharacter|Walk :!label _label))
  (:Released
    (goto _label Released)))

(event Input|ActionEvents|InputActionLightAttack
  (params (Key :type Key%20Structure :default "None"))
  ;[0 0 0] Attack
  (:Pressed
    (Class|PlayerCharacter|PlayerAttack "LightAttack")))

(event Input|ActionEvents|InputActionX-Ray
  (params (Key :type Key%20Structure :default "None"))
  ;[0 0 0] Lock On Target - Vision
  (:Pressed
    (Utilities|FlowControl|FlipFlop
      (:A
        (bind _parameter_value (Timeline|Timeline_0 Play)
          (:Update
            (Rendering|Material|SetScalarParameterValue "/Game/PlayerCharacter/VFX/LocationFinder/PC_Collection_PP.PC_Collection_PP" "Alpha" _parameter_value :!class /Script/Engine.KismetMaterialLibrary))))
      (:B
        (Timeline|Timeline_0 Reverse)))))

(event Input|ActionEvents|InputActionLockOnTarget
  (params (Key :type Key%20Structure :default "None"))
  ;[0 0 0] Lock On Target - Vision
  (:Pressed
    (Class|PlayerCharacter|LockonTarget)))

(event Input|AxisEvents|InputAxisFB
  (params (AxisValue :type Float%20%28single-precision%29))
  ;[0 0 0] FB - LR - Turn - LookUp
  (Class|PlayerCharacter|MoveCharacter AxisValue (Input|AxisValues|GetLR)))

(event Input|AxisEvents|InputAxisTurn
  (params (AxisValue :type Float%20%28single-precision%29))
  ;[0 0 0] FB - LR - Turn - LookUp
  (Class|PlayerCharacter|RotateCharacter AxisValue (Input|AxisValues|GetLookUp)))

(event Input|AxisEvents|InputAxisTurnGamePad
  (params (AxisValue :type Float%20%28single-precision%29))
  ;[0 0 0] FB - LR - Turn - LookUp
  (Class|PlayerCharacter|RotateCharacter AxisValue (Input|AxisValues|GetLookUpGamepad)))

(event Input|KeyboardEvents|1
  (params (Key :type Key%20Structure :default "None"))
  (:Pressed
    (Utilities|Time|SetGlobalTimeDilation 0.3)))

(event Input|KeyboardEvents|2
  (params (Key :type Key%20Structure :default "None"))
  (:Pressed
    (Utilities|Time|SetGlobalTimeDilation 1.0)))

(fn ConstructionScript)