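; BP_PlayerCharacter is the player character, handling movement, camera turning, light attack and an X-Ray toggle, and adding the main UI on BeginPlay.
; Axis inputs feed MoveCharacter and RotateCharacter, while Sprint and Walk forward press and release.
; The attack messages the AnimInstance through the MontagePlayer interface, gated by GetCanAttack.
; X-Ray flip-flops a timeline driving a parameter collection's Alpha, and construction registers the Weapon child actor.
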(event EventBeginPlay
  (bind _returnvalue (UserInterface|CreateWidget "/Game/Blueprints/UI/MainUIScreen.MainUIScreen_C"))
  (UserInterface|Viewport|AddtoViewport _returnvalue 0))

(event Input|ActionEvents|InputActionSprint
  (params (Key :type Key%20Structure :default "None"))
  (:Pressed
    (Class|PlayerCharacter|Sprint :!label _label))
  (:Released
    (goto _label Released)))

(event Input|ActionEvents|InputActionWalk
  (params (Key :type Key%20Structure :default "None"))
  (:Pressed
    (Class|PlayerCharacter|Walk :!label _label))
  (:Released
    (goto _label Released)))

(event Input|ActionEvents|InputActionLightAttack
  (params (Key :type Key%20Structure :default "None"))
  (:Pressed
    (bind _outputpin (Utilities|InterfaceCheck (Components|SkeletalMesh|GetAnimInstance (Variables|Character|GetMesh))))
    (Class|MontagePlayer|PlayMontage(Message) _outputpin "LightAttack")))

(event Input|ActionEvents|InputActionX-Ray
  (params (Key :type Key%20Structure :default "None"))
  (:Pressed
    (Utilities|FlowControl|FlipFlop
      (:A
        (bind _parameter_value (Timeline|Param%20Changer Play)
          (:Update
            (Rendering|Material|SetScalarParameterValue "/Game/VFX/LocationFinder/PC_Collection_PP.PC_Collection_PP" "Alpha" _parameter_value :!class /Script/Engine.KismetMaterialLibrary))))
      (:B
        (Timeline|Param%20Changer Reverse)))))

(event Input|AxisEvents|InputAxisFB
  (params (AxisValue :type Float%20%28single-precision%29))
  (Class|PlayerCharacter|MoveCharacter AxisValue (Input|AxisValues|GetLR)))

(event Input|AxisEvents|InputAxisTurn
  (params (AxisValue :type Float%20%28single-precision%29))
  (Class|PlayerCharacter|RotateCharacter AxisValue (Input|AxisValues|GetLookUp)))

(event Input|AxisEvents|InputAxisTurnGamePad
  (params (AxisValue :type Float%20%28single-precision%29))
  (Class|PlayerCharacter|RotateCharacter AxisValue (Input|AxisValues|GetLookUpGamepad)))

(fn ConstructionScript
  (bind _asbp_weapon_actor (Utilities|Casting|CastToBP_WeaponActor (Variables|/Script/Engine.ChildActorComponent|GetChildActor (Variables|Default|GetWeapon))))
  (Class|PlayerCharacter|SetWeaponActor _asbp_weapon_actor))