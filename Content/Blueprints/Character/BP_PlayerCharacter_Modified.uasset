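; Player character Blueprint that handles movement, camera turning and light melee attacks, and creates the main UI screen on BeginPlay.
; Axis inputs feed shared move and rotate functions, while sprint and walk actions forward press and release.
; Light attack messages the anim instance through the MontagePlayer interface, gated by CanAttack.
; The construction script caches the child-actor weapon for collision toggling, and a Debug function prints locomotion, action and ability states.
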(event EventBeginPlay
  (bind _returnvalue (UserInterface|CreateWidget "/Game/Blueprints/UI/MainUIScreen.MainUIScreen_C"))
  (UserInterface|Viewport|AddtoViewport _returnvalue 0))

(event EventChangeWeaponCollision
  (params (CollisionActive :type Boolean))
  (Default|ChangeCollision (Variables|Default|GetAs%20BP%20Weapon%20Actor) CollisionActive))

(event Input|ActionEvents|InputActionSprint
  (params (Key :type Key%20Structure))
  (:Pressed
    (Class|PlayerCharacter|Sprint :!label _label))
  (:Released
    (goto _label Released)))

(event Input|ActionEvents|InputActionWalk
  (params (Key :type Key%20Structure))
  (:Pressed
    (Class|PlayerCharacter|Walk :!label _label))
  (:Released
    (goto _label Released)))

(event Input|ActionEvents|InputActionLightAttack
  (params (Key :type Key%20Structure))
  (:Pressed
    (bind _outputpin (Utilities|InterfaceCheck (Components|SkeletalMesh|GetAnimInstance (Variables|Character|GetMesh))))
    (Class|MontagePlayer|PlayMontage(Message) _outputpin "LightAttack")))

(event Input|AxisEvents|InputAxisFB
  (params (AxisValue :type Float%20%28single-precision%29))
  (Class|PlayerCharacter|MoveCharacter AxisValue (Input|AxisValues|GetLR)))

(event Input|AxisEvents|InputAxisTurn
  (params (AxisValue :type Float%20%28single-precision%29))
  (Class|PlayerCharacter|RotateCharacter AxisValue (Input|AxisValues|GetLookUp)))

(event Input|AxisEvents|InputAxisTurnGamePad
  (params (AxisValue :type Float%20%28single-precision%29))
  (Class|PlayerCharacter|RotateCharacter AxisValue (Input|AxisValues|GetLookUpGamepad)))

(fn ConstructionScript
  (bind _asbp_weapon_actor (Utilities|Casting|CastToBP_WeaponActor (Variables|/Script/Engine.ChildActorComponent|GetChildActor (Variables|Default|GetWeapon))))
  (Variables|Default|SetAs%20BP%20Weapon%20Actor _asbp_weapon_actor))

(fn Debug
  (Development|PrintString (Utilities|String|Append "Locomotion: " (Utilities|String|EnumtoString (Variables|Default|GetLocomotionState))) true false "(R=0.000000,G=0.660000,B=1.000000,A=1.000000)" 0.0)
  (Development|PrintString (Utilities|String|Append "Action Mode: " (Utilities|String|EnumtoString (Variables|Default|GetActionState))) true false "(R=0.000000,G=0.660000,B=1.000000,A=1.000000)" 0.0)
  (Development|PrintString (Utilities|String|Append "Ability Mode: " (Utilities|String|EnumtoString (Variables|Default|GetAbilityState))) true false "(R=0.000000,G=0.660000,B=1.000000,A=1.000000)" 0.0))