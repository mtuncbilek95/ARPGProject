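; Anim notify state that manages attack rotation and combo state during a window of an animation.
; Each event messages the mesh's anim instance through the ComboSection interface, if implemented.
; Begin clears the next light and heavy combo sections, sets the attack flag and requests the combat rotation, which each tick then applies.
; End restores the opening combo sections and clears the attack flag.
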(fn ReceivedNotifyTick
  (params (MeshComp :type Skeletal%20Mesh%20Component%20Object%20Reference) (Animation :type Anim%20Sequence%20Base%20Object%20Reference) (FrameDeltaTime :type Float%20%28single-precision%29) (EventReference :type Anim%20Notify%20Event%20Reference%20Structure%20%28by%20ref%29))
  (bind _returnvalue (Components|SkeletalMesh|GetAnimInstance MeshComp))
  (if (Utilities|DoesObjectImplementInterface _returnvalue "/Script/SoulsProject.ComboSection")
    (Class|ComboSection|SetCombatRotation(Message) _returnvalue)
    (return false)))

(fn ReceivedNotifyBegin
  (params (MeshComp :type Skeletal%20Mesh%20Component%20Object%20Reference) (Animation :type Anim%20Sequence%20Base%20Object%20Reference) (TotalDuration :type Float%20%28single-precision%29) (EventReference :type Anim%20Notify%20Event%20Reference%20Structure%20%28by%20ref%29))
  (bind _returnvalue (Components|SkeletalMesh|GetAnimInstance MeshComp))
  (if (Utilities|DoesObjectImplementInterface _returnvalue "/Script/SoulsProject.ComboSection")
    (Class|ComboSection|NextCombo(Message) _returnvalue "None" "None")
    (Class|MontagePlayer|AttackSetter(Message) _returnvalue true)
    (Class|ComboSection|GetCombatRotation(Message) _returnvalue)
    (return true)))

(fn ReceivedNotifyEnd
  (params (MeshComp :type Skeletal%20Mesh%20Component%20Object%20Reference) (Animation :type Anim%20Sequence%20Base%20Object%20Reference) (EventReference :type Anim%20Notify%20Event%20Reference%20Structure%20%28by%20ref%29))
  (bind _returnvalue (Components|SkeletalMesh|GetAnimInstance MeshComp))
  (if (Utilities|DoesObjectImplementInterface _returnvalue "/Script/SoulsProject.ComboSection")
    (Class|ComboSection|NextCombo(Message) _returnvalue "Light1" "Heavy1")
    (Class|MontagePlayer|AttackSetter(Message) _returnvalue false)
    (return false)))